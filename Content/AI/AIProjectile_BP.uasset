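; AI projectile actor that damages AI characters and the player character on overlap, then destroys itself.
; An AI character is hit only through its capsule component, while any overlapping component of the player character counts.
; Each branch uses a DoOnce to apply fixed damage, passing the projectile's owner as damage causer.
; A short delay from BeginPlay destroys projectiles that hit nothing.
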(event OnComponentBeginOverlap(ProjectileOverlap)
  (params (OverlappedComponent :type Primitive%20Component%20Object%20Reference) (OtherActor :type Actor%20Object%20Reference) (OtherComp :type Primitive%20Component%20Object%20Reference) (OtherBodyIndex :type Integer) (bFromSweep :type Boolean) (SweepResult :type Hit%20Result%20Structure%20%28by%20ref%29))
  (bind _returnvalue (Components|GetOwner))
  (bind _asai_char_bp (Utilities|Casting|CastToAI_Char_BP OtherActor)
    (:then
      (if (== OtherComp (Variables|/Script/Engine.Character|GetCapsuleComponent _asai_char_bp))
        (Utilities|FlowControl|DoOnce false
          (:Completed
            (Game|Damage|ApplyDamage _asai_char_bp 1e+01 0 _returnvalue)
            (Actor|DestroyActor :!label _label)))))
    (:CastFailed
      (bind _asplayer_character_bp (Utilities|Casting|CastToPlayerCharacter_BP OtherActor))
      (Utilities|FlowControl|DoOnce false
        (:Completed
          (Game|Damage|ApplyDamage _asplayer_character_bp 1e+01 0 _returnvalue)
          (goto _label))))))

(event EventBeginPlay
  (Utilities|FlowControl|Delay 2.0)
  (Actor|DestroyActor))

(fn ConstructionScript)